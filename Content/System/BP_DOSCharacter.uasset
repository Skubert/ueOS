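; Player character that acts as the keyboard for a DOS-style terminal, creating the W_Screen widget on BeginPlay.
; Any key press is looked up in the Keys map, and its normal or shifted character, chosen by Caps Lock XOR Shift, is typed into the screen's last line.
; Backspace chops that line's final character, and Enter passes the last input's text to the screen's ParseCommand.
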(event EventBeginPlay
  (bind _returnvalue (UserInterface|CreateWidget "/UECLI/UI/W_Screen.W_Screen_C"))
  (UserInterface|Viewport|AddtoViewport _returnvalue 0)
  (Variables|Default|SetscreenRef _returnvalue))

(event Custom|InputChar
  (params (Char :type Key%20Structure :default "None"))
  (bind _screenref (Variables|Default|GetscreenRef))
  (bind _keys (Variables|Default|GetKeys))
  (bind _lines (Variables|/UECLI/UI/W_Screen.W_Screen_C|GetLines _screenref))
  (bind _returnvalue (Utilities|Array|LastIndex _lines))
  (bind _output (Utilities|Array|Get(acopy) _lines _returnvalue))
  ;[1 1 1] Adds a new character IF the key is in the Keys dictionary
  (bind _keys_2 (Utilities|Map|Keys _keys))
  (bind _values (Utilities|Map|Values _keys))
  (if (!= (Utilities|Array|FindItem _keys_2 Char) -1)
    (if (CallFunction|ShouldbeCaps)
      (Default|InputText _output (Utilities|Text|ToText(String) (.outshifted (Utilities|Array|Get(acopy) _values (Utilities|Array|FindItem _keys_2 Char)))))
      (else
        (Default|InputText _output (Utilities|Text|ToText(String) (.outnormal (Utilities|Array|Get(acopy) _values (Utilities|Array|FindItem _keys_2 Char)))))))))

(event Input|KeyboardEvents|Enter
  (params (Key :type Key%20Structure :default "None"))
  (bind _screenref (Variables|Default|GetscreenRef))
  (:Pressed
    (Default|ParseCommand _screenref (Utilities|String|ToString(Text) (Class|TextBlock|GetText (Variables|/UECLI/UI/W_Line.W_Line_C|GettextLine (Variables|/UECLI/UI/W_Screen.W_Screen_C|GetlastInput _screenref)))) false)))

(event Input|KeyboardEvents|Backspace
  (params (Key :type Key%20Structure :default "None"))
  (bind _screenref (Variables|Default|GetscreenRef))
  (bind _lines (Variables|/UECLI/UI/W_Screen.W_Screen_C|GetLines _screenref))
  (bind _returnvalue (Utilities|Array|LastIndex _lines))
  (bind _output (Utilities|Array|Get(acopy) _lines _returnvalue))
  (bind _textline (Variables|/UECLI/UI/W_Line.W_Line_C|GettextLine _output))
  (:Pressed
    (Rendering|Components|TextRender|SetText _textline (Utilities|Text|ToText(String) (Utilities|String|LeftChop (Utilities|String|ToString(Text) (Class|TextBlock|GetText _textline)) 1)))))

(event Input|KeyboardEvents|AnyKey
  (params (Key :type Key%20Structure :default "None"))
  ;[1 1 1] Adds a new character IF the key is in the Keys dictionary
  (:Pressed
    (CallFunction|InputChar Key)))

(fn ConstructionScript)

(fn IsShiftHeld
  (bind _returnvalue (Game|GetPlayerController 0))
  (return (or (Game|Player|IsInputKeyDown _returnvalue "RightShift") (Game|Player|IsInputKeyDown _returnvalue "LeftShift"))))

(fn ShouldbeCaps
  (return (Class|KismetMathLibrary|XORBoolean (Class|UECLIBPLibrary|AreCapsLocked) (CallFunction|IsShiftHeld))))

(fn GetHeldKeys
  (bind _keys (Variables|Default|GetKeys))
  (if (> (Utilities|Map|Length _keys) 0)
    (bind _values (Utilities|Map|Values _keys))
    (for _array_element _values
      (LocalVariables|SetNewLocalVar_0 (Utilities|String|Append (LocalVariables|GetNewLocalVar_0) (.outnormal _array_element)))
      (LocalVariables|SetNewLocalVar_1 (Utilities|String|Append (LocalVariables|GetNewLocalVar_1) (.outshifted _array_element)))))
  (return (LocalVariables|GetNewLocalVar_0) (LocalVariables|GetNewLocalVar_1)))