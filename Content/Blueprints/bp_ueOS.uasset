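; bp_ueOS turns raw key presses into typed characters and prints them as debug strings, apparently as keyboard input for an in-engine OS.
; Any non-special key is looked up in KeysTable, with ShiftTable supplying Shift variants.
; Keys missing from KeysTable fall back to their display name, cased by Shift and a Caps Lock flag that toggles on each press of that key.
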(event Input|KeyboardEvents|CapsLock
  (params (Key :type Key%20Structure))
  (:Pressed
    (Variables|Default|SetisCapsLockOn (not (Variables|Default|GetisCapsLockOn)))))

(event Input|KeyboardEvents|AnyKey
  (params (Key :type Key%20Structure))
  (bind _returnvalue (Class|KismetInputLibrary|KeyGetDisplayName Key))
  (bind _shifttable (Variables|Default|GetshiftTable))
  (bind _keystable (Variables|Default|GetkeysTable))
  (bind _shifttable_2 (Variables|Default|GetshiftTable))
  (bind (_value _returnvalue_2) (Utilities|Map|Find _shifttable Key))
  (bind _returnvalue_3 (Utilities|String|ToString(Text) _returnvalue))
  (bind (_value_2 _returnvalue_4) (Utilities|Map|Find _keystable Key))
  (bind (_value_3 _returnvalue_5) (Utilities|Map|Find _shifttable_2 Key))
  (bind _returnvalue_6 (Utilities|String|ToLower _returnvalue_3))
  (:Pressed
    (if (not (CallFunction|IsSpecialKey Key))
      (if _returnvalue_4
        (if (CallFunction|IsShiftDown)
          (Development|PrintString (select _returnvalue_2 _value _value_2))
          (else
            (Development|PrintString _value_2)))
        (elif (CallFunction|IsShiftDown)
          (Development|PrintString (select (Variables|Default|GetisCapsLockOn) _returnvalue_6 (select _returnvalue_5 _value_3 _returnvalue_3)))
          (else
            (Development|PrintString (select (Variables|Default|GetisCapsLockOn) _returnvalue_3 (select (CallFunction|IsLetter Key) _returnvalue_6 _returnvalue_3)))))))))

(fn ConstructionScript)